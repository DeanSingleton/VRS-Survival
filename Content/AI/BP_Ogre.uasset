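; Ogre enemy that jump-attacks the VR player, driven by a proximity sphere.
; A VRPawn entering the sphere sets IsInRange and plays a sound; any actor leaving triggers JumpAttack, with a delayed second sound for the pawn.
; JumpAttack plays a montage, sweeps the ogre to the player's capsule location, then after a short delay applies damage without rechecking range.
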(event OnComponentBeginOverlap(Sphere)
  (params (OverlappedComponent :type Primitive%20Component%20Object%20Reference) (OtherActor :type Actor%20Object%20Reference) (OtherComp :type Primitive%20Component%20Object%20Reference) (OtherBodyIndex :type Integer) (bFromSweep :type Boolean) (SweepResult :type Hit%20Result%20Structure%20%28by%20ref%29))
  (Utilities|Casting|CastToVRPawn OtherActor)
  (Variables|Default|SetIsInRange? true)
  (Audio|PlaySound2D "/Game/AudioAndSFX/CombatSFX/Wooden_Box_Destroy_02.Wooden_Box_Destroy_02" 1.0 1.0 0.0 0 0))

(event OnComponentEndOverlap(Sphere)
  (params (OverlappedComponent :type Primitive%20Component%20Object%20Reference) (OtherActor :type Actor%20Object%20Reference) (OtherComp :type Primitive%20Component%20Object%20Reference) (OtherBodyIndex :type Integer))
  (CallFunction|JumpAttack)
  (Utilities|Casting|CastToVRPawn OtherActor)
  (Utilities|FlowControl|Delay 1.0)
  (Audio|PlaySound2D "/Game/AudioAndSFX/GunsSFX/Ak47_Aiming_003.Ak47_Aiming_003" 1.0 1.0 0.0 0 0))

(event Custom|JumpAttack
  (bind _returnvalue (Game|GetPlayerCharacter 0))
  (bind _asvrpawn (Utilities|Casting|CastToVRPawn _returnvalue))
  (Animation|Montage|PlayMontage (Variables|Character|GetMesh) "/Game/AI/Ogre/Mutant_Jump_Attack_Montage.Mutant_Jump_Attack_Montage"
    (:then
      (Utilities|IsValid _asvrpawn
        (:Is%20Valid
          (Transformation|SetActorLocation (Transformation|GetWorldLocation (Variables|/Script/Engine.Character|GetCapsuleComponent _asvrpawn)) true false)
          (Utilities|FlowControl|Delay 0.5)
          (Default|TakeDamage _asvrpawn 1e+02))))))

(fn ConstructionScript)