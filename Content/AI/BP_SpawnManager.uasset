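; Wave manager that spawns enemies at typed spawner points and advances through numbered waves.
; On BeginPlay it sorts all BP_Spawner actors into melee, gun and ogre lists, then runs a short timer countdown.
; Each wave reads its data table row by wave number and spawns each enemy group at random matching points.
; A once-per-second poll detects when all spawned enemies are gone, plays a sound, then restarts the countdown for the next wave.
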(event Custom|StartCountdown
  ;[1 1 1] Countdown
  (bind _returnvalue (Utilities|Time|SetTimerbyEvent (delegate Custom|Count) 1.0 true))
  (Variables|Default|SetTime 3))

(event Custom|Count
  ;[1 1 1] Countdown
  (if (== (Variables|Default|GetTime) 0)
    (Utilities|Time|ClearandInvalidateTimerbyHandle (stale Custom|StartCountdown _returnvalue))
    (CallFunction|BeginWave)
    (else
      (Math|Integer|DecrementInt (Variables|Default|GetTime)))))

(event Custom|BeginWave
  ;[1 1 1] Spawn enemies for wave
  (bind _returnvalue (Utilities|GetDataTableRow (Variables|Default|GetEnemyDataTable) (Utilities|String|StringToName (Utilities|String|ToString(Integer) (Variables|Default|GetWaveNumber))))
    (:then
      (for _array_element (Utilities|Struct|BreakS_WaveInfo _returnvalue)
        (CallFunction|SpawnEnemies _array_element))
      (CallFunction|StartCheckingifEnemiesAreDead))))

(event Custom|StartCheckingIfEnemiesAreDead
  (bind _aredead_1 (CallFunction|CheckifAllEnemiesAreDead :!label _label))
  (if _aredead_1
    (Audio|SpawnSound2D "/Game/StarterContent/Audio/Explosion01.Explosion01" 1.0 1.0 0.0 0)
    (Utilities|FlowControl|Delay 5.0)
    (Math|Integer|IncrementInt (Variables|Default|GetWaveNumber)
      (:%20%20
        (CallFunction|StartCountdown)))
    (else
      (Utilities|FlowControl|Delay 1.0)
      (goto _label))))

(event EventBeginPlay
  (bind _outactors (Actor|GetAllActorsOfClass "/Game/AI/BP_Spawner.BP_Spawner_C"))
  (bind _output_get (Variables|Default|SetEnemySpawnPoints _outactors))
  (for _array_element _output_get
    (switch Utilities|FlowControl|Switch|SwitchonE_EnemyTypes (Variables|/Game/AI/BP_Spawner.BP_Spawner_C|GetSpawnerType _array_element)
      (:NewEnumerator0
        (Utilities|Array|Add (Variables|Default|GetE_Melee) _array_element))
      (:NewEnumerator1
        (Utilities|Array|Add (Variables|Default|GetE_Gun) _array_element))
      (:NewEnumerator4
        (Utilities|Array|Add (Variables|Default|GetE_Wendigo) _array_element))))
  (CallFunction|StartCountdown))

(fn ConstructionScript)

(fn SpawnEnemies
  (params (S_EnemyInfo :type S%20Enemy%20Info%20Structure%20%28by%20ref%29))
  (LocalVariables|SetEnemyInfoREF S_EnemyInfo)
  (LocalVariables|SetCurrentSpawnPoints (Utilities|Select :Index (.EnemyType (Utilities|Struct|BreakS_EnemyInfo S_EnemyInfo)) :NewEnumerator0 (Variables|Default|GetE_Melee) :NewEnumerator1 (Variables|Default|GetE_Gun) :NewEnumerator4 (Variables|Default|GetE_Wendigo)))
  (for _index (range 1 (.enemynumber (LocalVariables|GetEnemyInfoREF)))
    (bind _returnvalue (Game|SpawnActorfromClass (.enemyclass (LocalVariables|GetEnemyInfoREF)) (Transformation|GetWorldTransform (Variables|/Game/AI/BP_Spawner.BP_Spawner_C|GetBillboard (Utilities|Array|Get(acopy) (LocalVariables|GetCurrentSpawnPoints) (Math|Random|RandomIntegerinRange 0 (Utilities|Array|LastIndex (LocalVariables|GetCurrentSpawnPoints)))))) "AlwaysSpawn" 0 0))
    (Utilities|Array|Add (Variables|Default|GetCurrentEnemies) _returnvalue)))

(fn CheckifAllEnemiesAreDead
  (Variables|Default|SetAreDead? true)
  (for _array_element (Variables|Default|GetCurrentEnemies)
    (Utilities|IsValid _array_element
      (:Is%20Valid
        (Variables|Default|SetAreDead? false))))
  (return (Variables|Default|GetAreDead?)))