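; Cultist enemy for a VR wave game that attacks the player and planks, counting itself in VRGameMode's EnemiesAlive.
; Capsule overlap starts looping timers for montage-driven player damage and plank damage; end overlap never clears them.
; DealDamage computes Health as Damage minus Health (reversed subtraction); death updates the GameMode, destroys the actor and awards points.
; AIJump wraps Jump; several older attack chains remain disconnected.
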(event OnComponentBeginOverlap(Capsule)
  (params (OverlappedComponent :type Primitive%20Component%20Object%20Reference) (OtherActor :type Actor%20Object%20Reference) (OtherComp :type Primitive%20Component%20Object%20Reference) (OtherBodyIndex :type Integer) (bFromSweep :type Boolean) (SweepResult :type Hit%20Result%20Structure%20%28by%20ref%29))
  (Utilities|FlowControl|Sequence
    (:then_0
      (Utilities|Time|SetTimerbyEvent (delegate Custom|Attack) 2.0 true))
    (:then_1
      (Utilities|Time|SetTimerbyEvent (delegate Custom|RemovePlank) 1.0 true))))

(event OnComponentEndOverlap(Capsule)
  (params (OverlappedComponent :type Primitive%20Component%20Object%20Reference) (OtherActor :type Actor%20Object%20Reference) (OtherComp :type Primitive%20Component%20Object%20Reference) (OtherBodyIndex :type Integer))
  (Variables|Default|SetAttacking? false))

(event Custom|AIJump
  (Character|Jump))

(event Custom|Attack
  (bind _asvrpawn (Utilities|Casting|CastToVRPawn (stale OnComponentBeginOverlap(Capsule) OtherActor)))
  (Animation|Montage|PlayMontage (Variables|Character|GetMesh) "/Game/AI/Culstist/Anims/Zombie_Attack_Montage.Zombie_Attack_Montage"
    (:then
      (Utilities|IsValid _asvrpawn
        (:Is%20Valid
          (Default|TakeDamage _asvrpawn 2e+01))))))

(event Custom|RemovePlank
  (bind _asplank (Utilities|Casting|CastToPlank (stale OnComponentBeginOverlap(Capsule) OtherActor)))
  (if (Variables|/Game/Programming/Blueprints/VRInventorySystem/Items/Plank.Plank_C|GetPlaced? _asplank)
    (Utilities|IsValid _asplank
      (:Is%20Valid
        (Default|TakeDamage _asplank 5e+01)
        (Utilities|IsValid _asplank
          (:Is%20Valid
            (Default|Destroyed _asplank)))))))

(event EventDealDamage
  (params (Damage :type Float%20%28double-precision%29))
  (bind _output_get (Variables|Default|SetHealth (- Damage (Variables|Default|GetHealth))))
  (if (<= _output_get 0.0)
    (Development|PrintString "Enemy Died")
    (bind _asvrgame_mode (Utilities|Casting|CastToVRGameMode (Game|GetGameMode)))
    (Math|Integer|DecrementInt (Variables|/Game/VRTemplate/Blueprints/VRGameMode.VRGameMode_C|GetEnemiesAlive _asvrgame_mode)
      (:%20%20
        (Default|CheckEnemiesLeft _asvrgame_mode)
        (Actor|DestroyActor)
        (bind _asvrpawn (Utilities|Casting|CastToVRPawn (Game|GetPlayerCharacter 0)))
        (Default|AddPoints _asvrpawn (Variables|Default|GetPointsGiven))))
    (else
      (Development|PrintString (Utilities|String|ToString(Float) _output_get)))))

(event EventBeginPlay
  (bind _asvrgame_mode (Utilities|Casting|CastToVRGameMode (Game|GetGameMode)))
  (Math|Integer|IncrementInt (Variables|/Game/VRTemplate/Blueprints/VRGameMode.VRGameMode_C|GetEnemiesAlive _asvrgame_mode)))

(fn ConstructionScript)