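; Boss Blueprint with a jump attack that teleports it onto the player's VRPawn and deals area damage.
; Any actor leaving its Sphere triggers the attack; a VRPawn entering sets IsInRange, and both crossings play sounds for VRPawns.
; JumpAttack plays a montage, moves to the player's capsule, then after a short delay damages VRPawns found by a WorldStatic-only sphere overlap, drawn with a debug sphere.
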(event OnComponentBeginOverlap(Sphere)
  (params (OverlappedComponent :type Primitive%20Component%20Object%20Reference) (OtherActor :type Actor%20Object%20Reference) (OtherComp :type Primitive%20Component%20Object%20Reference) (OtherBodyIndex :type Integer) (bFromSweep :type Boolean) (SweepResult :type Hit%20Result%20Structure%20%28by%20ref%29))
  (Utilities|Casting|CastToVRPawn OtherActor)
  (Variables|Default|SetIsInRange? true)
  (Audio|PlaySound2D "/Game/AudioAndSFX/CombatSFX/Wooden_Box_Destroy_02.Wooden_Box_Destroy_02" 1.0 1.0 0.0 0 0))

(event OnComponentEndOverlap(Sphere)
  (params (OverlappedComponent :type Primitive%20Component%20Object%20Reference) (OtherActor :type Actor%20Object%20Reference) (OtherComp :type Primitive%20Component%20Object%20Reference) (OtherBodyIndex :type Integer))
  (CallFunction|JumpAttack)
  (Utilities|Casting|CastToVRPawn OtherActor)
  (Utilities|FlowControl|Delay 1.0)
  (Audio|PlaySound2D "/Game/AudioAndSFX/GunsSFX/Ak47_Aiming_003.Ak47_Aiming_003" 1.0 1.0 0.0 0 0))

(event Custom|JumpAttack
  (bind _returnvalue (Transformation|GetActorLocation))
  (bind _returnvalue_2 (Game|GetPlayerCharacter 0))
  (bind _asvrpawn (Utilities|Casting|CastToVRPawn _returnvalue_2))
  (Animation|Montage|PlayMontage (Variables|Character|GetMesh) "/Game/AI/Culstist/Anims/Jump_Attack_Montage.Jump_Attack_Montage"
    (:then
      (Utilities|IsValid _asvrpawn
        (:Is%20Valid
          (Transformation|SetActorLocation (Transformation|GetWorldLocation (Variables|/Script/Engine.Character|GetCapsuleComponent _asvrpawn)) false false)
          (Utilities|FlowControl|Delay 0.5)
          (bind _outactors (Collision|SphereOverlapActors _returnvalue (Variables|Default|GetBlastRadius) (Utilities|Array|MakeArray "ObjectTypeQuery1") 0))
          (Rendering|Debug|DrawDebugSphere _returnvalue (Variables|Default|GetBlastRadius) 12 "(R=1.000000,G=0.000000,B=0.000000,A=1.000000)" 3.0 2.0)
          ;[1 1 1] What happens to actors inside blast radius
          (for _array_element _outactors
            (bind _asvrpawn_2 (Utilities|Casting|CastToVRPawn _array_element))
            (Default|TakeDamage _asvrpawn_2 3e+01)))))))

(fn ConstructionScript)