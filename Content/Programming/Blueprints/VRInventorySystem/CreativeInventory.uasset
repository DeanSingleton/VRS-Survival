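; CreativeInventory is a VR inventory actor that acts as a spawner for a configurable actor class, handing out a fresh copy on each grab.
; On BeginPlay it spawns a scaled, collision-free preview of that class attached to its static mesh.
; When its GrabComponent is grabbed, it spawns a new instance at its own transform and passes the motion controller to that instance's GrabComponent through TryGrab.
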(event OnGrabbed(GrabComponent)
  (bind _returnvalue (Game|SpawnActorfromClass (Variables|Default|GetActorClass) (Transformation|GetActorTransform) "AlwaysSpawn" 0 0))
  (Utilities|IsValid (Actor|GetComponentbyClass _returnvalue "/Game/Programming/Blueprints/VRInventorySystem/GrabComponent.GrabComponent_C")
    (:Is%20Valid
      (Default|TryGrab (Actor|GetComponentbyClass _returnvalue "/Game/Programming/Blueprints/VRInventorySystem/GrabComponent.GrabComponent_C") (Variables|/Game/Programming/Blueprints/VRInventorySystem/GrabComponent.GrabComponent_C|GetMotionControllerRef (Variables|Default|GetGrabComponent))))))

(event EventBeginPlay
  (bind _returnvalue (Game|SpawnActorfromClass (Variables|Default|GetActorClass) (Math|Transform|MakeTransform "0, 0, 0" "0, 0, 0" "1.000000,1.000000,1.000000") "AlwaysSpawn" 0 0))
  (Transformation|AttachComponentToComponent _returnvalue (Variables|Default|GetStaticMesh) "None" "SnapToTarget" "SnapToTarget" "KeepWorld" true)
  (Transformation|SetActorScale3D _returnvalue (Variables|Default|GetPreviewScale))
  (Collision|SetActorEnableCollision _returnvalue false))

(fn ConstructionScript)