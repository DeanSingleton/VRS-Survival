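; VR inventory component that stores loose grabbable items where they are dropped inside its overlap volume.
; While Active, each tick attaches previously held targets that were released, keeping world transform, then re-sorts overlapping GrabComponent actors into held targets and contained items.
; Held targets swap in an overlap highlight material.
; HideActors feeds one boolean to both the contained actors' hidden state and Active, so hiding them enables processing.
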(event EventBeginPlay
  (Variables|Default|SetOriginalMaterial (Rendering|Material|GetMaterial 0)))

(event EventTick
  (params (DeltaSeconds :type Float%20%28single-precision%29))
  (bind _overlappedmaterial (Variables|Default|GetOverlappedMaterial))
  (if (Variables|Default|GetActive?)
    (Utilities|FlowControl|Sequence
      (:then_0
        (for _array_element (Variables|Default|GetTargetActors)
          (if (not (Variables|/Game/Programming/Blueprints/VRInventorySystem/GrabComponent.GrabComponent_C|GetbIsHeld (Actor|GetComponentbyClass _array_element "/Game/Programming/Blueprints/VRInventorySystem/GrabComponent.GrabComponent_C")))
            (Transformation|AttachComponentToComponent _array_element self "None" "KeepWorld" "KeepWorld" "KeepWorld" true))))
      (:then_1
        (Utilities|Array|Clear (Variables|Default|GetTargetActors))
        (Utilities|Array|Clear (Variables|Default|GetContainedActors))
        (for _array_element_2 (Collision|GetOverlappingActors 0 :!class /Script/Engine.PrimitiveComponent)
          (Utilities|IsValid (Actor|GetComponentbyClass _array_element_2 "/Game/Programming/Blueprints/VRInventorySystem/GrabComponent.GrabComponent_C")
            (:Is%20Valid
              (if (Variables|/Game/Programming/Blueprints/VRInventorySystem/GrabComponent.GrabComponent_C|GetbIsHeld (Actor|GetComponentbyClass _array_element_2 "/Game/Programming/Blueprints/VRInventorySystem/GrabComponent.GrabComponent_C"))
                (Utilities|Array|Add (Variables|Default|GetTargetActors) _array_element_2)
                (Utilities|IsValid _overlappedmaterial
                  (:Is%20Valid
                    (Rendering|Material|SetMaterial 0 _overlappedmaterial)))
                (else
                  (Utilities|Array|Add (Variables|Default|GetContainedActors) _array_element_2))))))
        (if (== (Utilities|Array|Length (Variables|Default|GetTargetActors)) 0)
          (Rendering|Material|SetMaterial 0 (Variables|Default|GetOriginalMaterial)))))))

(fn HideActors
  (params (Visibility :type Boolean))
  (for _array_element (Variables|Default|GetContainedActors)
    (Rendering|SetActorHiddenInGame _array_element Visibility))
  (Variables|Default|SetActive? Visibility))