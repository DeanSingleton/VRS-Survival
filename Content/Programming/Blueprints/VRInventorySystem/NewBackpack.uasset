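; VR inventory backpack actor that stays invisible until grabbed and holds four NewHolster child-actor slots.
; On grab it snaps to the grabbing motion controller, shows and shadows its mesh, and clears each holster's Hidden flag.
; On drop, if DefaultComponent is valid, it snaps back there and hides mesh and holsters again.
; Active reports whether the pack is out; the Grab and Release events are empty.
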(event OnGrabbed(GrabComponent)
  (Transformation|DetachFromComponent (Variables|Default|GetDefaultSceneRoot) "KeepRelative" "KeepRelative" "KeepRelative" true)
  (Transformation|AttachComponentToComponent (Variables|/Game/Programming/Blueprints/VRInventorySystem/GrabComponent.GrabComponent_C|GetMotionControllerRef (Variables|Default|GetGrabComponent)) "None" "SnapToTarget" "SnapToTarget" "KeepWorld" true)
  (Development|SetHiddeninGame (Variables|Default|GetStaticMesh) false true)
  (Rendering|SetCastShadow (Variables|Default|GetStaticMesh) true)
  (Variables|Default|SetActivated? true)
  (bind _asnew_holster (Utilities|Casting|CastToNewHolster (Variables|/Script/Engine.ChildActorComponent|GetChildActor (Variables|Default|GetInventorySlot1))))
  (Variables|/Game/Programming/Blueprints/VRWeaponSystem/Holsters/NewHolster.NewHolster_C|SetHidden? _asnew_holster false)
  (bind _asnew_holster_2 (Utilities|Casting|CastToNewHolster (Variables|/Script/Engine.ChildActorComponent|GetChildActor (Variables|Default|GetInventorySlot2))))
  (Variables|/Game/Programming/Blueprints/VRWeaponSystem/Holsters/NewHolster.NewHolster_C|SetHidden? _asnew_holster_2 false)
  (bind _asnew_holster_3 (Utilities|Casting|CastToNewHolster (Variables|/Script/Engine.ChildActorComponent|GetChildActor (Variables|Default|GetInventorySlot3))))
  (Variables|/Game/Programming/Blueprints/VRWeaponSystem/Holsters/NewHolster.NewHolster_C|SetHidden? _asnew_holster_3 false)
  (bind _asnew_holster_4 (Utilities|Casting|CastToNewHolster (Variables|/Script/Engine.ChildActorComponent|GetChildActor (Variables|Default|GetInventorySlot))))
  (Variables|/Game/Programming/Blueprints/VRWeaponSystem/Holsters/NewHolster.NewHolster_C|SetHidden? _asnew_holster_4 false))

(event OnDropped(GrabComponent)
  (bind _defaultcomponent (Variables|Default|GetDefaultComponent)
    (:then
      (Transformation|AttachComponentToComponent _defaultcomponent "None" "SnapToTarget" "SnapToTarget" "KeepWorld" true)
      (Development|SetHiddeninGame (Variables|Default|GetStaticMesh) true true)
      (Rendering|SetCastShadow (Variables|Default|GetStaticMesh) false)
      (Variables|Default|SetActivated? false)
      (bind _asnew_holster (Utilities|Casting|CastToNewHolster (Variables|/Script/Engine.ChildActorComponent|GetChildActor (Variables|Default|GetInventorySlot1))))
      (Variables|/Game/Programming/Blueprints/VRWeaponSystem/Holsters/NewHolster.NewHolster_C|SetHidden? _asnew_holster true)
      (bind _asnew_holster_2 (Utilities|Casting|CastToNewHolster (Variables|/Script/Engine.ChildActorComponent|GetChildActor (Variables|Default|GetInventorySlot2))))
      (Variables|/Game/Programming/Blueprints/VRWeaponSystem/Holsters/NewHolster.NewHolster_C|SetHidden? _asnew_holster_2 true)
      (bind _asnew_holster_3 (Utilities|Casting|CastToNewHolster (Variables|/Script/Engine.ChildActorComponent|GetChildActor (Variables|Default|GetInventorySlot3))))
      (Variables|/Game/Programming/Blueprints/VRWeaponSystem/Holsters/NewHolster.NewHolster_C|SetHidden? _asnew_holster_3 true)
      (bind _asnew_holster_4 (Utilities|Casting|CastToNewHolster (Variables|/Script/Engine.ChildActorComponent|GetChildActor (Variables|Default|GetInventorySlot))))
      (Variables|/Game/Programming/Blueprints/VRWeaponSystem/Holsters/NewHolster.NewHolster_C|SetHidden? _asnew_holster_4 true))
    (:else)))

(event EventGrab
  (params (MotionController :type Motion%20Controller%20Component%20Object%20Reference)))

(event EventRelease
  (params (MotionController :type Motion%20Controller%20Component%20Object%20Reference)))

(fn ConstructionScript
  (Development|SetHiddeninGame (Variables|Default|GetStaticMesh) true true))

(fn Active
  (return (Variables|Default|GetActivated?)))