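; TallGrass is a stealth-system actor that acts as a hiding zone for the first-person character.
; Its Box overlap events set the character's InGrass flag on entry and clear both InGrass and Hidden on exit.
; Hidden is set only if the character is already crouching on entry, with debug strings printing the result.
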(event OnComponentBeginOverlap(Box)
  (params (OverlappedComponent :type Primitive%20Component%20Object%20Reference) (OtherActor :type Actor%20Object%20Reference) (OtherComp :type Primitive%20Component%20Object%20Reference) (OtherBodyIndex :type Integer) (bFromSweep :type Boolean) (SweepResult :type Hit%20Result%20Structure%20%28by%20ref%29))
  (bind _asfirst_person_character (Utilities|Casting|CastToFirstPersonCharacter OtherActor))
  (Variables|/Game/Programming/Blueprints/Character/FirstPersonCharacter.FirstPersonCharacter_C|SetInGrass? _asfirst_person_character true)
  (if (Variables|/Game/Programming/Blueprints/Character/FirstPersonCharacter.FirstPersonCharacter_C|GetCrouching? _asfirst_person_character)
    (Variables|/Game/Programming/Blueprints/Character/FirstPersonCharacter.FirstPersonCharacter_C|SetHidden? _asfirst_person_character true)
    (Development|PrintString "Hidden")
    (else
      (Development|PrintString "NotHidden"))))

(event OnComponentEndOverlap(Box)
  (params (OverlappedComponent :type Primitive%20Component%20Object%20Reference) (OtherActor :type Actor%20Object%20Reference) (OtherComp :type Primitive%20Component%20Object%20Reference) (OtherBodyIndex :type Integer))
  (bind _asfirst_person_character (Utilities|Casting|CastToFirstPersonCharacter OtherActor))
  (Variables|/Game/Programming/Blueprints/Character/FirstPersonCharacter.FirstPersonCharacter_C|SetInGrass? _asfirst_person_character false)
  (Variables|/Game/Programming/Blueprints/Character/FirstPersonCharacter.FirstPersonCharacter_C|SetHidden? _asfirst_person_character false)
  (Development|PrintString "NotHidden"))

(event EventBeginPlay)

(event Collision|EventActorBeginOverlap
  (params (OtherActor :type Actor%20Object%20Reference)))

(event EventTick
  (params (DeltaSeconds :type Float%20%28single-precision%29)))

(fn ConstructionScript)