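; PlankSlot is a crafting-system slot that decides when an overlapping Plank can be placed.
; Left and right collision volumes each set their own flag when a Plank enters, and the Plank becomes Placeable only when both flags are set.
; A Plank leaving either side clears that flag, loses Placeable and is Reset.
; The flags track sides only, not which Plank set them.
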(event OnComponentBeginOverlap(LeftSideCollision)
  (params (OverlappedComponent :type Primitive%20Component%20Object%20Reference) (OtherActor :type Actor%20Object%20Reference) (OtherComp :type Primitive%20Component%20Object%20Reference) (OtherBodyIndex :type Integer) (bFromSweep :type Boolean) (SweepResult :type Hit%20Result%20Structure%20%28by%20ref%29))
  (bind _asplank (Utilities|Casting|CastToPlank OtherActor))
  (Utilities|IsValid _asplank
    (:Is%20Valid
      (Variables|Default|SetLeftCheck? true)
      (if (and (Variables|Default|GetLeftCheck?) (Variables|Default|GetRightCheck?))
        (Variables|/Game/Programming/Blueprints/VRInventorySystem/Items/Plank.Plank_C|SetPlaceable? _asplank true)
        (else
          (Variables|/Game/Programming/Blueprints/VRInventorySystem/Items/Plank.Plank_C|SetPlaceable? _asplank false))))))

(event OnComponentEndOverlap(LeftSideCollision)
  (params (OverlappedComponent :type Primitive%20Component%20Object%20Reference) (OtherActor :type Actor%20Object%20Reference) (OtherComp :type Primitive%20Component%20Object%20Reference) (OtherBodyIndex :type Integer))
  (bind _asplank (Utilities|Casting|CastToPlank OtherActor))
  (Variables|Default|SetLeftCheck? false)
  (Variables|/Game/Programming/Blueprints/VRInventorySystem/Items/Plank.Plank_C|SetPlaceable? _asplank false)
  (Default|Reset _asplank))

(event OnComponentBeginOverlap(RightSideCollision)
  (params (OverlappedComponent :type Primitive%20Component%20Object%20Reference) (OtherActor :type Actor%20Object%20Reference) (OtherComp :type Primitive%20Component%20Object%20Reference) (OtherBodyIndex :type Integer) (bFromSweep :type Boolean) (SweepResult :type Hit%20Result%20Structure%20%28by%20ref%29))
  (bind _asplank (Utilities|Casting|CastToPlank OtherActor))
  (Utilities|IsValid _asplank
    (:Is%20Valid
      (Variables|Default|SetRightCheck? true)
      (if (and (Variables|Default|GetLeftCheck?) (Variables|Default|GetRightCheck?))
        (Variables|/Game/Programming/Blueprints/VRInventorySystem/Items/Plank.Plank_C|SetPlaceable? _asplank true)
        (else
          (Variables|/Game/Programming/Blueprints/VRInventorySystem/Items/Plank.Plank_C|SetPlaceable? _asplank false))))))

(event OnComponentEndOverlap(RightSideCollision)
  (params (OverlappedComponent :type Primitive%20Component%20Object%20Reference) (OtherActor :type Actor%20Object%20Reference) (OtherComp :type Primitive%20Component%20Object%20Reference) (OtherBodyIndex :type Integer))
  (bind _asplank (Utilities|Casting|CastToPlank OtherActor))
  (Variables|Default|SetRightCheck? false)
  (Variables|/Game/Programming/Blueprints/VRInventorySystem/Items/Plank.Plank_C|SetPlaceable? _asplank false)
  (Default|Reset _asplank))

(fn ConstructionScript)