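; SinglePlankSlot is a crafting system actor that marks where a Plank can be placed.
; When a Plank begins overlapping its OverlapCollision, the slot sets OverlapCheck and flags that plank as Placeable.
; When the overlap ends, it clears both flags and calls Reset on the plank.
; The slot does no placing or snapping itself, only toggling state on the overlapping Plank.
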(event OnComponentBeginOverlap(OverlapCollision)
  (params (OverlappedComponent :type Primitive%20Component%20Object%20Reference) (OtherActor :type Actor%20Object%20Reference) (OtherComp :type Primitive%20Component%20Object%20Reference) (OtherBodyIndex :type Integer) (bFromSweep :type Boolean) (SweepResult :type Hit%20Result%20Structure%20%28by%20ref%29))
  (bind _asplank (Utilities|Casting|CastToPlank OtherActor))
  (Utilities|IsValid _asplank
    (:Is%20Valid
      (bind _output_get (Variables|Default|SetOverlapCheck? true))
      (if _output_get
        (Variables|/Game/Programming/Blueprints/VRInventorySystem/Items/Plank.Plank_C|SetPlaceable? _asplank true)
        (else
          (Variables|/Game/Programming/Blueprints/VRInventorySystem/Items/Plank.Plank_C|SetPlaceable? _asplank false))))))

(event OnComponentEndOverlap(OverlapCollision)
  (params (OverlappedComponent :type Primitive%20Component%20Object%20Reference) (OtherActor :type Actor%20Object%20Reference) (OtherComp :type Primitive%20Component%20Object%20Reference) (OtherBodyIndex :type Integer))
  (bind _asplank (Utilities|Casting|CastToPlank OtherActor))
  (if true
    (Variables|Default|SetOverlapCheck? false)
    (Variables|/Game/Programming/Blueprints/VRInventorySystem/Items/Plank.Plank_C|SetPlaceable? _asplank false)
    (Default|Reset _asplank)))

(fn ConstructionScript)