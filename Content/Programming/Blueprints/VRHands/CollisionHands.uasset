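; Physics-driven VR hands actor whose left and right skeletal meshes follow the motion controllers.
; SetUp stores references to both motion controllers and has a Physics Handle grab each hand mesh at its current transform.
; Every Tick moves each handle's target to its controller's location and rotation, so the hands are pulled along through physics instead of being attached directly.
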(event EventTick
  (params (DeltaSeconds :type Float%20%28single-precision%29))
  (bind _rightmotioncontroller (Variables|Default|GetRightMotionController))
  (bind _leftmotioncontroller (Variables|Default|GetLeftMotionController))
  (bind _returnvalue (Transformation|GetWorldTransform _rightmotioncontroller))
  (bind _returnvalue_2 (Transformation|GetWorldTransform _leftmotioncontroller))
  (Class|PhysicsHandleComponent|SetTargetLocationandRotation (Variables|Default|GetPhysicsHandleLeft) (.location _returnvalue_2) (.rotation _returnvalue_2))
  (Class|PhysicsHandleComponent|SetTargetLocationandRotation (Variables|Default|GetPhysicsHandleRight) (.location _returnvalue) (.rotation _returnvalue)))

(fn ConstructionScript)

(fn SetUp
  (params (LeftMotionController :type Motion%20Controller%20Component%20Object%20Reference) (RightMotionController :type Motion%20Controller%20Component%20Object%20Reference))
  (bind _skeletalmeshleft (Variables|Default|GetSkeletalMeshLeft))
  (bind _skeletalmeshright (Variables|Default|GetSkeletalMeshRight))
  (bind _returnvalue (Transformation|GetWorldTransform _skeletalmeshleft))
  (bind _returnvalue_2 (Transformation|GetWorldTransform _skeletalmeshright))
  (Variables|Default|SetLeftMotionController LeftMotionController)
  (Variables|Default|SetRightMotionController RightMotionController)
  (Physics|Components|PhysicsHandle|GrabComponentatLocationwithRotation (Variables|Default|GetPhysicsHandleLeft) _skeletalmeshleft "None" (.location _returnvalue) (.rotation _returnvalue))
  (Physics|Components|PhysicsHandle|GrabComponentatLocationwithRotation (Variables|Default|GetPhysicsHandleRight) _skeletalmeshright "None" (.location _returnvalue_2) (.rotation _returnvalue_2)))